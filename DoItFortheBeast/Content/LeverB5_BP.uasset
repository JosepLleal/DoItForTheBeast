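; Interactable lever actor that can only be pulled once its Completed flag is true, which this graph reads but never sets.
; A trigger box enables input and custom-depth highlighting when the first-person character enters, and disables both on end overlap.
; Interact plays a sound and a timeline-driven roll: either a full pull that sets LeverPulled when finished, or a stuck animation replayed from the start.
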(event `self.box.OnComponentBeginOverlap`
  (params (OverlappedComponent :type "PrimitiveComponent Object Reference") (OtherActor :type "Actor Object Reference") (OtherComp :type "PrimitiveComponent Object Reference") (OtherBodyIndex :type Integer) (bFromSweep :type Boolean) (SweepResult :type "HitResult Structure (by ref)"))
  ;[1 1 1] Enable/Disable Input
  (bind _asfirst_person_character (cast `/Game/FirstPersonBP/Blueprints/FirstPersonCharacter` OtherActor))
  (set `self.As First Person Character` _asfirst_person_character)
  (`self.EnableInput` (`GameplayStatics.GetPlayerController` 0))
  (`PrimitiveComponent.SetRenderCustomDepth` (`self.lever`) true))

(event `self.box.OnComponentEndOverlap`
  (params (OverlappedComponent :type "PrimitiveComponent Object Reference") (OtherActor :type "Actor Object Reference") (OtherComp :type "PrimitiveComponent Object Reference") (OtherBodyIndex :type Integer))
  ;[1 1 1] Enable/Disable Input
  (`self.DisableInput` (`GameplayStatics.GetPlayerController` 0))
  (`PrimitiveComponent.SetRenderCustomDepth` (`self.lever`) false))

(event `InputAction|Interact`
  (params (Key :type "Key Structure"))
  (bind _lever (`self.lever`))
  (:`Pressed`
    (if (`self.Completed`)
      (`GameplayStatics.PlaySoundAtLocation` "/Game/Assets/Audio/Lever.Lever" (0.0 0.0 0.0) (struct) 1.0 1.0 0.0 null null null)
      (bind (_direction _levermovement) (`Timeline|Timeline_0`)
        (:`Update`
          (`SceneComponent.K2_SetRelativeRotation` _lever (`KismetMathLibrary.MakeRotator` _levermovement) false false))
        (:`Finished`
          (set `self.Lever Pulled` true)))
      (else
        (`GameplayStatics.PlaySoundAtLocation` "/Game/Assets/Audio/leverStuck.leverStuck" (0.0 0.0 0.0) (struct) 1.0 1.0 0.0 null null null)
        (bind (_direction_2 _levermovement_2) (`Timeline|Timeline_1` :!via `PlayFromStart`)
          (:`Update`
            (`SceneComponent.K2_SetRelativeRotation` _lever (`KismetMathLibrary.MakeRotator` _levermovement_2) false false)))))))

(fn `UserConstructionScript`)