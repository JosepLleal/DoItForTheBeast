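; Balance scale puzzle prop where the player places or retrieves heart and diamond items on two plates.
; Box overlaps highlight the plate with custom depth and enable input, so E moves items between the character's OwnedKeys and that plate, toggling preplaced meshes.
; Each change picks a preset rotation from the plate contents, then a timeline lerps the pole to it while both plates follow their joints to world positions.
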(event `self.BoxPlate1.OnComponentBeginOverlap`
  (params (OverlappedComponent :type "PrimitiveComponent Object Reference") (OtherActor :type "Actor Object Reference") (OtherComp :type "PrimitiveComponent Object Reference") (OtherBodyIndex :type Integer) (bFromSweep :type Boolean) (SweepResult :type "HitResult Structure (by ref)"))
  ;[1 1 1] Overlap Trigger Boxes
  (bind _asfirst_person_character (cast `/Game/FirstPersonBP/Blueprints/FirstPersonCharacter` OtherActor))
  (set `self.As First Person Character` _asfirst_person_character)
  (`PrimitiveComponent.SetRenderCustomDepth` (`self.Plate1`) true)
  (`PrimitiveComponent.SetRenderCustomDepth` (`self.Heart1`) true)
  (`PrimitiveComponent.SetRenderCustomDepth` (`self.Diamond1`) true)
  (set `self.OnPlate1` true)
  (`self.EnableInput` (`GameplayStatics.GetPlayerController` 0)))

(event `self.BoxPlate1.OnComponentEndOverlap`
  (params (OverlappedComponent :type "PrimitiveComponent Object Reference") (OtherActor :type "Actor Object Reference") (OtherComp :type "PrimitiveComponent Object Reference") (OtherBodyIndex :type Integer))
  ;[1 1 1] Overlap Trigger Boxes
  (`PrimitiveComponent.SetRenderCustomDepth` (`self.Plate1`) false)
  (`PrimitiveComponent.SetRenderCustomDepth` (`self.Heart1`) false)
  (`PrimitiveComponent.SetRenderCustomDepth` (`self.Diamond1`) false)
  (set `self.OnPlate1` false)
  (`self.DisableInput` (`GameplayStatics.GetPlayerController` 0)))

(event `self.BoxPlate2.OnComponentBeginOverlap`
  (params (OverlappedComponent :type "PrimitiveComponent Object Reference") (OtherActor :type "Actor Object Reference") (OtherComp :type "PrimitiveComponent Object Reference") (OtherBodyIndex :type Integer) (bFromSweep :type Boolean) (SweepResult :type "HitResult Structure (by ref)"))
  ;[1 1 1] Overlap Trigger Boxes
  (bind _asfirst_person_character (cast `/Game/FirstPersonBP/Blueprints/FirstPersonCharacter` OtherActor))
  (set `self.As First Person Character` _asfirst_person_character)
  (`PrimitiveComponent.SetRenderCustomDepth` (`self.Plate2`) true)
  (`PrimitiveComponent.SetRenderCustomDepth` (`self.Heart2`) true)
  (`PrimitiveComponent.SetRenderCustomDepth` (`self.Diamond2`) true)
  (set `self.OnPlate2` true)
  (`self.EnableInput` (`GameplayStatics.GetPlayerController` 0)))

(event `self.BoxPlate2.OnComponentEndOverlap`
  (params (OverlappedComponent :type "PrimitiveComponent Object Reference") (OtherActor :type "Actor Object Reference") (OtherComp :type "PrimitiveComponent Object Reference") (OtherBodyIndex :type Integer))
  ;[1 1 1] Overlap Trigger Boxes
  (`PrimitiveComponent.SetRenderCustomDepth` (`self.Plate2`) false)
  (`PrimitiveComponent.SetRenderCustomDepth` (`self.Heart2`) false)
  (`PrimitiveComponent.SetRenderCustomDepth` (`self.Diamond2`) false)
  (set `self.OnPlate2` false)
  (`self.DisableInput` (`GameplayStatics.GetPlayerController` 0)))

(event `Key|E`
  (params (Key :type "Key Structure"))
  (bind _objectonplate1 (`self.ObjectOnPlate1`))
  (bind _objectonplate2 (`self.ObjectOnPlate2`))
  (bind _ownedkeys (`/Game/FirstPersonBP/Blueprints/FirstPersonCharacter.OwnedKeys` (`self.As First Person Character`)))
  (bind _ownedkeys_2 (`/Game/FirstPersonBP/Blueprints/FirstPersonCharacter.OwnedKeys` (`self.As First Person Character`)))
  (:`Pressed`
    (if (`self.OnPlate1`)
      ;[1 1 1] Plate 1
      (if (`|EnumEquality` (`self.ObjectOnPlate1`) "NewEnumerator0")
        (for _array_element (`/Game/FirstPersonBP/Blueprints/FirstPersonCharacter.OwnedKeys` (`self.As First Person Character`))
          (if (`|EnumEquality` _array_element "NewEnumerator9")
            (`SceneComponent.SetVisibility` (`self.Heart1`) true false)
            (bind _output_get (set `self.ObjectOnPlate1` "NewEnumerator9"))
            (`KismetArrayLibrary.Array_RemoveItem` _ownedkeys_2 _output_get)
            (`self.Scale Balance` :!label _label)
            (`self.Move Scale`)))
        (if (`|EnumEquality` (`self.ObjectOnPlate1`) "NewEnumerator0")
          (for _array_element_2 _ownedkeys_2
            (if (`|EnumEquality` _array_element_2 "NewEnumerator10")
              (`SceneComponent.SetVisibility` (`self.Diamond1`) true false)
              (bind _output_get_2 (set `self.ObjectOnPlate1` "NewEnumerator10"))
              (`KismetArrayLibrary.Array_RemoveItem` _ownedkeys_2 _output_get_2)
              (goto _label))))
        (else
          (`KismetArrayLibrary.Array_Add` (`/Game/FirstPersonBP/Blueprints/FirstPersonCharacter.OwnedKeys` (`self.As First Person Character`)) _objectonplate1)
          (if (`|EnumEquality` _objectonplate1 "NewEnumerator9")
            (`SceneComponent.SetVisibility` (`self.Heart1`) false false)
            (set `self.ObjectOnPlate1` "NewEnumerator0" :!label _label_2)
            (goto _label)
            (elif (`|EnumEquality` _objectonplate1 "NewEnumerator10")
              (`SceneComponent.SetVisibility` (`self.Diamond1`) false false)
              (goto _label_2)))))
      (elif (`self.OnPlate2`)
        ;[1 1 1] Plate 2
        (if (`|EnumEquality` (`self.ObjectOnPlate2`) "NewEnumerator0")
          (for _array_element_3 (`/Game/FirstPersonBP/Blueprints/FirstPersonCharacter.OwnedKeys` (`self.As First Person Character`))
            (if (`|EnumEquality` _array_element_3 "NewEnumerator9")
              (`SceneComponent.SetVisibility` (`self.Heart2`) true false)
              (bind _output_get_3 (set `self.ObjectOnPlate2` "NewEnumerator9"))
              (`KismetArrayLibrary.Array_RemoveItem` _ownedkeys _output_get_3)
              (goto _label)))
          (if (`|EnumEquality` (`self.ObjectOnPlate2`) "NewEnumerator0")
            (for _array_element_4 _ownedkeys
              (if (`|EnumEquality` _array_element_4 "NewEnumerator10")
                (`SceneComponent.SetVisibility` (`self.Diamond2`) true false)
                (bind _output_get_4 (set `self.ObjectOnPlate2` "NewEnumerator10"))
                (`KismetArrayLibrary.Array_RemoveItem` _ownedkeys _output_get_4)
                (goto _label))))
          (else
            (`KismetArrayLibrary.Array_Add` (`/Game/FirstPersonBP/Blueprints/FirstPersonCharacter.OwnedKeys` (`self.As First Person Character`)) _objectonplate2)
            (if (`|EnumEquality` _objectonplate2 "NewEnumerator9")
              (`SceneComponent.SetVisibility` (`self.Heart2`) false false)
              (set `self.ObjectOnPlate2` "NewEnumerator0" :!label _label_3)
              (goto _label)
              (elif (`|EnumEquality` _objectonplate2 "NewEnumerator10")
                (`SceneComponent.SetVisibility` (`self.Diamond2`) false false)
                (goto _label_3)))))))))

(event `Scale Balance`
  ;[1 1 1] Set Scale New Rotation
  (if (and (`|EnumEquality` (`self.ObjectOnPlate1`) "NewEnumerator0") (`|EnumEquality` (`self.ObjectOnPlate2`) "NewEnumerator0"))
    (set `self.NewRotation` 0)
    (elif (and (`|EnumEquality` (`self.ObjectOnPlate1`) "NewEnumerator9") (`|EnumEquality` (`self.ObjectOnPlate2`) "NewEnumerator0"))
      (set `self.NewRotation` 2)
      (elif (and (`|EnumEquality` (`self.ObjectOnPlate1`) "NewEnumerator0") (`|EnumEquality` (`self.ObjectOnPlate2`) "NewEnumerator9"))
        (set `self.NewRotation` 4)
        (elif (and (`|EnumEquality` (`self.ObjectOnPlate1`) "NewEnumerator10") (`|EnumEquality` (`self.ObjectOnPlate2`) "NewEnumerator0"))
          (set `self.NewRotation` 2)
          (elif (and (`|EnumEquality` (`self.ObjectOnPlate1`) "NewEnumerator0") (`|EnumEquality` (`self.ObjectOnPlate2`) "NewEnumerator10"))
            (set `self.NewRotation` 4)
            (elif (and (`|EnumEquality` (`self.ObjectOnPlate1`) "NewEnumerator9") (`|EnumEquality` (`self.ObjectOnPlate2`) "NewEnumerator10"))
              (set `self.NewRotation` 1)
              (elif (and (`|EnumEquality` (`self.ObjectOnPlate1`) "NewEnumerator10") (`|EnumEquality` (`self.ObjectOnPlate2`) "NewEnumerator9"))
                (set `self.NewRotation` 3)))))))))

(event `Move Scale`
  ;[1 1 1] Move Scale Event
  (set `self.LastRotation` (`SceneComponent.RelativeRotation` (`self.Pole2`)))
  (bind (_direction _value) (`Timeline|Timeline_0` :!via `PlayFromStart`)
    (:`Update`
      (`SceneComponent.K2_SetRelativeRotation` (`self.Pole2`) (`KismetMathLibrary.RLerp` (`self.LastRotation`) (`|GetArrayItem` (`self.RotationsArray`) (`self.NewRotation`)) _value true) false false)
      (`SceneComponent.K2_SetWorldLocation` (`self.MovePlate1`) (`SceneComponent.K2_GetComponentLocation` (`self.PlateJoint1`)) false false)
      (`SceneComponent.K2_SetWorldLocation` (`self.MovePlate2`) (`SceneComponent.K2_GetComponentLocation` (`self.PlateJoint2`)) false false))))

(fn `UserConstructionScript`)