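; Interactable note actor that the first-person character can read by pressing E while standing near it.
; Entering its Box enables input and turns on the note mesh's custom depth as a highlight; any end overlap reverses both.
; E creates one of six note widgets chosen by the NoteType enum.
; All branches share one AddToViewport step, which then pauses the game and shows the mouse cursor.
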(event `self.Box.OnComponentBeginOverlap`
  (params (OverlappedComponent :type "PrimitiveComponent Object Reference") (OtherActor :type "Actor Object Reference") (OtherComp :type "PrimitiveComponent Object Reference") (OtherBodyIndex :type Integer) (bFromSweep :type Boolean) (SweepResult :type "HitResult Structure (by ref)"))
  ;[1 1 1] Enable/Disable Input
  (bind _asfirst_person_character (cast `/Game/FirstPersonBP/Blueprints/FirstPersonCharacter` OtherActor))
  (set `self.As First Person Character` _asfirst_person_character)
  (`self.EnableInput` (`GameplayStatics.GetPlayerController` 0))
  (`PrimitiveComponent.SetRenderCustomDepth` (`self.Note`) true))

(event `self.Box.OnComponentEndOverlap`
  (params (OverlappedComponent :type "PrimitiveComponent Object Reference") (OtherActor :type "Actor Object Reference") (OtherComp :type "PrimitiveComponent Object Reference") (OtherBodyIndex :type Integer))
  ;[1 1 1] Enable/Disable Input
  (`self.DisableInput` (`GameplayStatics.GetPlayerController` 0))
  (`PrimitiveComponent.SetRenderCustomDepth` (`self.Note`) false))

(event `Key|E`
  (params (Key :type "Key Structure"))
  (:`Pressed`
    (if (`|EnumEquality` (`self.Note_Type`) "NewEnumerator0")
      (bind _returnvalue (`|CreateWidget` "/Game/PauseMenu/Note_B1.Note_B1_C"))
      (`UserWidget.AddToViewport` (stale _returnvalue_2) 0 :!label _label)
      (`UserWidget.AddToViewport` (stale _returnvalue_3) 0)
      (`UserWidget.AddToViewport` _returnvalue 0)
      (`UserWidget.AddToViewport` (stale _returnvalue_4) 0)
      (`UserWidget.AddToViewport` (stale _returnvalue_5) 0)
      (`UserWidget.AddToViewport` (stale _returnvalue_6) 0)
      (`GameplayStatics.SetGamePaused` true)
      (set `PlayerController.bShowMouseCursor` true (`GameplayStatics.GetPlayerController` 0))
      (elif (`|EnumEquality` (`self.Note_Type`) "NewEnumerator1")
        (bind _returnvalue_2 (`|CreateWidget` "/Game/PauseMenu/Note_B5.Note_B5_C"))
        (goto _label)
        (elif (`|EnumEquality` (`self.Note_Type`) "NewEnumerator2")
          (bind _returnvalue_3 (`|CreateWidget` "/Game/PauseMenu/Note_B6.Note_B6_C"))
          (goto _label)
          (elif (`|EnumEquality` (`self.Note_Type`) "NewEnumerator3")
            (bind _returnvalue_4 (`|CreateWidget` "/Game/PauseMenu/Note_B9.Note_B9_C"))
            (goto _label)
            (elif (`|EnumEquality` (`self.Note_Type`) "NewEnumerator4")
              (bind _returnvalue_5 (`|CreateWidget` "/Game/PauseMenu/Note_B12.Note_B12_C"))
              (goto _label)
              (elif (`|EnumEquality` (`self.Note_Type`) "NewEnumerator5")
                (bind _returnvalue_6 (`|CreateWidget` "/Game/PauseMenu/Note_B13.Note_B13_C"))
                (goto _label)))))))))

(fn `UserConstructionScript`)