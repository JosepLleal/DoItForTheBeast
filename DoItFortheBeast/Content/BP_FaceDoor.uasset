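; BP_FaceDoor is a key-locked door that lights an eye and moves open when the player uses the required key.
; A sphere overlap caches the FirstPersonCharacter, enables input and outlines the door through custom depth; end overlap reverses input and highlight.
; Pressing E while closed plays a crumble sound, then searches OwnedKeys for RequiredKeyType.
; A match marks it open, shows RightEye and, after a delay, runs the DoorMovement timeline.
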(event `self.Sphere.OnComponentBeginOverlap`
  (params (OverlappedComponent :type "PrimitiveComponent Object Reference") (OtherActor :type "Actor Object Reference") (OtherComp :type "PrimitiveComponent Object Reference") (OtherBodyIndex :type Integer) (bFromSweep :type Boolean) (SweepResult :type "HitResult Structure (by ref)"))
  ;[1 1 1] Enable/Disable Input
  (bind _asfirst_person_character (cast `/Game/FirstPersonBP/Blueprints/FirstPersonCharacter` OtherActor))
  (set `self.As First Person Character` _asfirst_person_character)
  (`self.EnableInput` (`GameplayStatics.GetPlayerController` 0))
  (`PrimitiveComponent.SetRenderCustomDepth` (`self.Door`) true))

(event `self.Sphere.OnComponentEndOverlap`
  (params (OverlappedComponent :type "PrimitiveComponent Object Reference") (OtherActor :type "Actor Object Reference") (OtherComp :type "PrimitiveComponent Object Reference") (OtherBodyIndex :type Integer))
  ;[1 1 1] Enable/Disable Input
  (`self.DisableInput` (`GameplayStatics.GetPlayerController` 0))
  (`PrimitiveComponent.SetRenderCustomDepth` (`self.Door`) false))

(event `Key|E`
  (params (Key :type "Key Structure"))
  (bind _door (`self.Door`))
  (:`Pressed`
    (if (`self.DoorIsClosed`)
      (`GameplayStatics.PlaySoundAtLocation` "/Game/Assets/Audio/rock_Crumble.rock_Crumble" (0.0 0.0 0.0) (struct) 0.3 1.0 1.0 null null null)
      (for _array_element (`/Game/FirstPersonBP/Blueprints/FirstPersonCharacter.OwnedKeys` (`self.As First Person Character`))
        (if (`|EnumEquality` _array_element (`self.RequiredKeyType`))
          (set `self.DoorIsClosed` false)
          (`SceneComponent.SetVisibility` (`self.RightEye`) true false)
          (`KismetSystemLibrary.Delay` 2.0)
          (bind (_direction _up) (`Timeline|Door Movement`)
            (:`Update`
              (`SceneComponent.K2_SetRelativeTransform` _door (`KismetMathLibrary.MakeTransform` _up (struct) (`SceneComponent.RelativeScale3D` _door)) false false))))))))

(fn `UserConstructionScript`)