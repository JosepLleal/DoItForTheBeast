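; Statue3_BP is an interactable statue that accepts one required object from the player's inventory.
; Entering its box as the first-person character enables input and turns on custom-depth rendering on the statue, and leaving turns both off.
; Pressing Interact searches the character's OwnedKeys for the required object, removes it, reveals the placed Object mesh, marks the statue filled and plays a placement sound.
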(event `self.Box.OnComponentBeginOverlap`
  (params (OverlappedComponent :type "PrimitiveComponent Object Reference") (OtherActor :type "Actor Object Reference") (OtherComp :type "PrimitiveComponent Object Reference") (OtherBodyIndex :type Integer) (bFromSweep :type Boolean) (SweepResult :type "HitResult Structure (by ref)"))
  ;[1 1 1] Disable/Enable Input
  (bind _asfirst_person_character (cast `/Game/FirstPersonBP/Blueprints/FirstPersonCharacter` OtherActor))
  (set `self.As First Person Character` _asfirst_person_character)
  (`self.EnableInput` (`GameplayStatics.GetPlayerController` 0))
  (`PrimitiveComponent.SetRenderCustomDepth` (`self.Statue`) true))

(event `self.Box.OnComponentEndOverlap`
  (params (OverlappedComponent :type "PrimitiveComponent Object Reference") (OtherActor :type "Actor Object Reference") (OtherComp :type "PrimitiveComponent Object Reference") (OtherBodyIndex :type Integer))
  ;[1 1 1] Disable/Enable Input
  (`self.DisableInput` (`GameplayStatics.GetPlayerController` 0))
  (`PrimitiveComponent.SetRenderCustomDepth` (`self.Statue`) false))

(event `InputAction|Interact`
  (params (Key :type "Key Structure"))
  (bind _ownedkeys (`/Game/FirstPersonBP/Blueprints/FirstPersonCharacter.OwnedKeys` (`self.As First Person Character`)))
  (:`Pressed`
    (if (not (`self.Has Object`))
      (for _array_element _ownedkeys
        (if (`|EnumEquality` _array_element (`self.Required Object`))
          (`KismetArrayLibrary.Array_RemoveItem` _ownedkeys _array_element)
          (`SceneComponent.SetVisibility` (`self.Object`) true false)
          (set `self.Has Object` true)
          (`GameplayStatics.PlaySound2D` "/Game/Assets/Audio/place_obj.place_obj" 1.0 1.0 0.0 null null))))))

(fn `UserConstructionScript`)