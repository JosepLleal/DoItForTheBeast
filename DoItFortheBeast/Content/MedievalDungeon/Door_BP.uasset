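; Door blueprint for a medieval dungeon that the player opens and closes with the Interact input.
; A box collision overlap enables input from player controller 0 and turns on custom depth on the door mesh, and leaving it reverses both.
; Each press plays a metal fence sound and toggles DoorClosed, playing or reversing the OpenCloseDoor timeline that drives the door's relative yaw.
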(event `self.BoxCollision.OnComponentBeginOverlap`
  (params (OverlappedComponent :type "PrimitiveComponent Object Reference") (OtherActor :type "Actor Object Reference") (OtherComp :type "PrimitiveComponent Object Reference") (OtherBodyIndex :type Integer) (bFromSweep :type Boolean) (SweepResult :type "HitResult Structure (by ref)"))
  ;[1 1 1] Enable/Disable Input
  (`self.EnableInput` (`GameplayStatics.GetPlayerController` 0))
  (`PrimitiveComponent.SetRenderCustomDepth` (`self.Door`) true))

(event `self.BoxCollision.OnComponentEndOverlap`
  (params (OverlappedComponent :type "PrimitiveComponent Object Reference") (OtherActor :type "Actor Object Reference") (OtherComp :type "PrimitiveComponent Object Reference") (OtherBodyIndex :type Integer))
  ;[1 1 1] Enable/Disable Input
  (`self.DisableInput` (`GameplayStatics.GetPlayerController` 0))
  (`PrimitiveComponent.SetRenderCustomDepth` (`self.Door`) false))

(event `InputAction|Interact`
  (params (Key :type "Key Structure"))
  ;[1 1 1] Open/Close Door
  (:`Pressed`
    (`GameplayStatics.PlaySoundAtLocation` "/Game/Assets/Audio/metal_fence.metal_fence" (0.0 0.0 0.0) (struct) 0.4 1.0 0.0 null null null)
    (if (`self.Door_Closed`)
      (set `self.Door_Closed` false)
      (bind (_direction _open_close_door) (`Timeline|Open/Close Door` :!label _label)
        (:`Update`
          (`SceneComponent.K2_SetRelativeRotation` (`self.Door`) (`KismetMathLibrary.MakeRotator` 0.0 0.0 _open_close_door) false false)))
      (else
        (set `self.Door_Closed` true)
        (goto _label :!via `Reverse`)))))

(fn `UserConstructionScript`)