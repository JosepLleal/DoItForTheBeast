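; WoodPlank_BP is an interactable pickup that adds its KeyType to the first-person character's OwnedKeys.
; Overlapping its Box with that character stores the reference, enables input and turns on custom depth for both wood meshes.
; Leaving the box disables input and custom depth.
; Pressing Interact adds the key, plays a wood or rock grab sound based on KeyType, then destroys the actor.
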(event `self.Box.OnComponentBeginOverlap`
  (params (OverlappedComponent :type "PrimitiveComponent Object Reference") (OtherActor :type "Actor Object Reference") (OtherComp :type "PrimitiveComponent Object Reference") (OtherBodyIndex :type Integer) (bFromSweep :type Boolean) (SweepResult :type "HitResult Structure (by ref)"))
  ;[1 1 1] Enable/Disable Input
  (bind _asfirst_person_character (cast `/Game/FirstPersonBP/Blueprints/FirstPersonCharacter` OtherActor))
  (set `self.As First Person Character` _asfirst_person_character)
  (`self.EnableInput` (`GameplayStatics.GetPlayerController` 0))
  (`PrimitiveComponent.SetRenderCustomDepth` (`self.Wood`) true)
  (`PrimitiveComponent.SetRenderCustomDepth` (`self.Wood1`) true))

(event `self.Box.OnComponentEndOverlap`
  (params (OverlappedComponent :type "PrimitiveComponent Object Reference") (OtherActor :type "Actor Object Reference") (OtherComp :type "PrimitiveComponent Object Reference") (OtherBodyIndex :type Integer))
  ;[1 1 1] Enable/Disable Input
  (`self.DisableInput` (`GameplayStatics.GetPlayerController` 0))
  (`PrimitiveComponent.SetRenderCustomDepth` (`self.Wood`) false)
  (`PrimitiveComponent.SetRenderCustomDepth` (`self.Wood1`) false))

(event `InputAction|Interact`
  (params (Key :type "Key Structure"))
  (bind _key_type (`self.Key Type`))
  (:`Pressed`
    (`KismetArrayLibrary.Array_Add` (`/Game/FirstPersonBP/Blueprints/FirstPersonCharacter.OwnedKeys` (`self.As First Person Character`)) _key_type)
    (if (or (`|EnumEquality` _key_type "NewEnumerator2") (`|EnumEquality` _key_type "NewEnumerator1"))
      (`GameplayStatics.PlaySound2D` "/Game/Assets/Audio/takewood.takewood" 1.0 1.0 0.0 null null)
      (else
        (`GameplayStatics.PlaySound2D` "/Game/Assets/Audio/grab_rocks.grab_rocks" 1.0 1.0 0.0 null null)))
    (`self.K2_DestroyActor`)))

(fn `UserConstructionScript`)