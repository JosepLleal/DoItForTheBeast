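; Interactive door test Blueprint that steps a Door component through eight preset rotations on repeated E presses.
; A box collision enables player input on begin overlap and disables it on end overlap.
; Each press increments a click counter to select the next target rotation, wrapping after the eighth.
; The OpenCloseDoor timeline replays from start, lerping relative rotation from the current value to the target by shortest path.
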(event `self.BoxCollision.OnComponentBeginOverlap`
  (params (OverlappedComponent :type "PrimitiveComponent Object Reference") (OtherActor :type "Actor Object Reference") (OtherComp :type "PrimitiveComponent Object Reference") (OtherBodyIndex :type Integer) (bFromSweep :type Boolean) (SweepResult :type "HitResult Structure (by ref)"))
  ;[1 1 1] Enable/Disable Input
  (`self.EnableInput` (`GameplayStatics.GetPlayerController` 0)))

(event `self.BoxCollision.OnComponentEndOverlap`
  (params (OverlappedComponent :type "PrimitiveComponent Object Reference") (OtherActor :type "Actor Object Reference") (OtherComp :type "PrimitiveComponent Object Reference") (OtherBodyIndex :type Integer))
  ;[1 1 1] Enable/Disable Input
  (`self.DisableInput` (`GameplayStatics.GetPlayerController` 0)))

(event `Key|E`
  (params (Key :type "Key Structure"))
  ;[1 1 1] Open/Close Door
  (:`Pressed`
    (set `self.LastRotation` (`SceneComponent.RelativeRotation` (`self.Door`)))
    (set `self.CLicks` (+ (`self.CLicks`) 1))
    (if (== (`self.CLicks`) 1)
      (set `self.Rotation_to_make` (`self.Rotation_01`))
      (bind (_direction _newtrack_1) (`Timeline|Open/Close Door` :!via `PlayFromStart` :!label _label)
        (:`Update`
          (`SceneComponent.K2_SetRelativeRotation` (`self.Door`) (`KismetMathLibrary.RLerp` (`self.LastRotation`) (`self.Rotation_to_make`) _newtrack_1 true) false false)))
      (elif (== (`self.CLicks`) 2)
        (set `self.Rotation_to_make` (`self.Rotation_02`))
        (goto _label :!via `PlayFromStart`)
        (elif (== (`self.CLicks`) 3)
          (set `self.Rotation_to_make` (`self.Rotation_03`))
          (goto _label :!via `PlayFromStart`)
          (elif (== (`self.CLicks`) 4)
            (set `self.Rotation_to_make` (`self.Rotation_04`))
            (goto _label :!via `PlayFromStart`)
            (elif (== (`self.CLicks`) 5)
              (set `self.Rotation_to_make` (`self.Rotation_05`))
              (goto _label :!via `PlayFromStart`)
              (elif (== (`self.CLicks`) 6)
                (set `self.Rotation_to_make` (`self.Rotation_06`))
                (goto _label :!via `PlayFromStart`)
                (elif (== (`self.CLicks`) 7)
                  (set `self.Rotation_to_make` (`self.Rotation_07`))
                  (goto _label :!via `PlayFromStart`)
                  (elif (== (`self.CLicks`) 8)
                    (set `self.Rotation_to_make` (`self.Rotation_08`))
                    (set `self.CLicks` 0)
                    (goto _label :!via `PlayFromStart`)))))))))))

(fn `UserConstructionScript`)