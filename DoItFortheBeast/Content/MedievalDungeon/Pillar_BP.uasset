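; Rotatable dungeon pillar that stays locked until the StatuesCompleted event lowers its metal bars.
; A box overlap toggles player input and a custom depth highlight on the pillar.
; StatuesCompleted plays a sound and a timeline that drops the four sticks and sets SticksDown.
; Pressing E then cycles a wrapping index through preset rotations, with a timeline lerping the root by the shortest path.
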(event `self.Box.OnComponentBeginOverlap`
  (params (OverlappedComponent :type "PrimitiveComponent Object Reference") (OtherActor :type "Actor Object Reference") (OtherComp :type "PrimitiveComponent Object Reference") (OtherBodyIndex :type Integer) (bFromSweep :type Boolean) (SweepResult :type "HitResult Structure (by ref)"))
  ;[1 1 1] Enable?disable Input
  (`self.EnableInput` (`GameplayStatics.GetPlayerController` 0))
  (`PrimitiveComponent.SetRenderCustomDepth` (`self.Pillar`) true))

(event `self.Box.OnComponentEndOverlap`
  (params (OverlappedComponent :type "PrimitiveComponent Object Reference") (OtherActor :type "Actor Object Reference") (OtherComp :type "PrimitiveComponent Object Reference") (OtherBodyIndex :type Integer))
  ;[1 1 1] Enable?disable Input
  (`self.DisableInput` (`GameplayStatics.GetPlayerController` 0))
  (`PrimitiveComponent.SetRenderCustomDepth` (`self.Pillar`) false))

(event `self.ReceiveBeginPlay`
  (bind _sticks (`self.Sticks`))
  ;[1 1 1] Get sticks into an array
  (`KismetArrayLibrary.Array_Add` _sticks (`self.MetalStick1`))
  (`KismetArrayLibrary.Array_Add` _sticks (`self.MetalStick4`))
  (`KismetArrayLibrary.Array_Add` _sticks (`self.MetalStick6`))
  (`KismetArrayLibrary.Array_Add` _sticks (`self.MetalStick8`)))

(event `Statues COmpleted`
  ;[1 1 1] Statues Completed Function
  (`GameplayStatics.PlaySoundAtLocation` "/Game/Assets/Audio/metalbarsdown.metalbarsdown" (0.0 0.0 0.0) (struct) 1.0 1.0 0.0 null null null)
  (bind (_direction _value) (`Timeline|Bars Down` :!via `PlayFromStart`)
    (:`Update`
      (for _array_element (`self.Sticks`)
        (bind (_relativelocation_x _relativelocation_y) (`KismetMathLibrary.BreakVector` (`SceneComponent.RelativeLocation` _array_element)))
        (`SceneComponent.K2_SetRelativeLocation` _array_element (`KismetMathLibrary.VLerp` (`KismetMathLibrary.MakeVector` _relativelocation_x _relativelocation_y) (+ (`KismetMathLibrary.MakeVector` _relativelocation_x _relativelocation_y) (0.0 0.0 -445.0)) _value) false false)
        (set `self.SticksDown` true)))))

(event `Key|E`
  (params (Key :type "Key Structure"))
  (bind _clicks (`self.Clicks`))
  ;[1 1 1] Interact with pillar
  (:`Pressed`
    (if (`self.SticksDown`)
      (set `self.Last Rotation` (`SceneComponent.RelativeRotation` (`self.DefaultSceneRoot`)))
      (set `self.Clicks` (+ _clicks 1))
      (if (not (!= _clicks 8))
        (set `self.Clicks` 0))
      (set `self.New Rotation` (`|GetArrayItem` (`self.mRotationArray`) (`self.Clicks`)))
      (`GameplayStatics.PlaySoundAtLocation` "/Game/Assets/Audio/coluimn_Rotation.coluimn_Rotation" (0.0 0.0 0.0) (struct) 1.0 1.0 0.0 null null null)
      (bind (_direction _value) (`Timeline|Rotate` :!via `PlayFromStart`)
        (:`Update`
          (`SceneComponent.K2_SetRelativeRotation` (`self.DefaultSceneRoot`) (`KismetMathLibrary.RLerp` (`self.Last Rotation`) (`self.New Rotation`) _value true) false false))))))

(fn `UserConstructionScript`)